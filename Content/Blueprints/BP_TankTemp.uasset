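; Player-controlled tank Blueprint that drives, fires, and offers orbit-style look controls with switchable first- and third-person cameras.
; Input forwards movement and firing to TankMovement and TankAiming components, which receive the tracks, barrel and turret on BeginPlay.
; Look yaw and pitch rotate separate Horizontal and SpringArm components.
; BeginPlay also sets the tank as owner of its UI_TankHealth widget.
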(event EventBeginPlay
  (Class|TankAimingComponent|SetBarrelandTurret (Variables|Default|GetTankAiming) (Variables|Default|GetBarrel) (Variables|Default|GetTurret))
  (Class|TankMovementComponent|SetTankTracks (Variables|Default|GetTankMovement) (Variables|Default|GetRight%20Track) (Variables|Default|GetLeft%20Track))
  (CallFunction|InitializeHealthbar))

(event Input|ActionEvents|InputActionFire
  (params (Key :type Key%20Structure))
  (:Pressed
    (Class|TankAimingComponent|Fire (Variables|Default|GetTankAiming))))

(event Input|ActionEvents|InputActionSwapCamera
  (params (Key :type Key%20Structure))
  (:Pressed
    (Components|Activation|ToggleActive (Variables|Default|GetFirst%20Person))
    (Components|Activation|ToggleActive (Variables|Default|GetThird%20Person))))

(event Input|AxisEvents|InputAxisHorizontalAxis
  (params (AxisValue :type Float%20%28single-precision%29))
  (Transformation|AddLocalRotation (Variables|Default|GetHorizontal) (Math|Rotator|MakeRotator 0.0 0.0 AxisValue) false false))

(event Input|AxisEvents|InputAxisVerticalAxis
  (params (AxisValue :type Float%20%28single-precision%29))
  (Transformation|AddLocalRotation (Variables|Default|GetSpringArm) (Math|Rotator|MakeRotator 0.0 AxisValue 0.0) false false))

(event Input|AxisEvents|InputAxisMoveForward
  (params (AxisValue :type Float%20%28single-precision%29))
  (Class|TankMovementComponent|MoveForward (Variables|Default|GetTankMovement) AxisValue))

(event Input|AxisEvents|InputAxisMoveRight
  (params (AxisValue :type Float%20%28single-precision%29))
  (Class|TankMovementComponent|MoveRight (Variables|Default|GetTankMovement) AxisValue))

(fn ConstructionScript)

(fn InitializeHealthbar
  (bind _asui_tank_health (Utilities|Casting|CastToUI_TankHealth (UserInterface|GetUserWidgetObject (Variables|Default|GetWidget))))
  (Variables|/Game/Blueprints/UI_TankHealth.UI_TankHealth_C|SetTank%20Owner _asui_tank_health self))