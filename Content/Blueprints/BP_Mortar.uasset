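; BP_Mortar is a mortar unit that reuses the tank aiming component and tank health bar widget.
; On BeginPlay it passes its barrel and turret to TankAiming, then initializes the health bar.
; The initialization casts the Widget component's user widget to UI_TankHealth and sets the mortar as its TankOwner.
; The Blueprint contains only this setup, with an empty construction script and no aiming or firing logic.
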(event EventBeginPlay
  (Class|TankAimingComponent|SetBarrelandTurret (Variables|Default|GetTankAiming) (Variables|Default|GetMortar%20Barrel) (Variables|Default|GetMortar%20Turret))
  (CallFunction|HealthbarInitialization))

(fn ConstructionScript)

(fn HealthbarInitialization
  (bind _asui_tank_health (Utilities|Casting|CastToUI_TankHealth (UserInterface|GetUserWidgetObject (Variables|Default|GetWidget))))
  (Variables|/Game/Blueprints/UI_TankHealth.UI_TankHealth_C|SetTank%20Owner _asui_tank_health self))